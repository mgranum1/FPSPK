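; BP_EnemyCharacter is an enemy character in the MonsterBear folder that shoots projectiles and has adjustable walk speed.
; ShootingPlayer plays the gunplay montage, then on completion spawns BP_Projectile at the mesh's GunSocket along control rotation, with itself as instigator.
; ShootPlayer only plays the same montage, without spawning a projectile.
; UpdateWalkSpeed sets the movement component's max walk speed.
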(event Custom|ShootingPlayer
  (Animation|Montage|PlayMontage (Variables|Character|GetMesh) "/Game/FPSPK/Enemies/MonsterBear/Animations/AM_EnemyCharacter_Gunplay_Montage.AM_EnemyCharacter_Gunplay_Montage"
    (:OnCompleted
      (Game|SpawnActorfromClass "/Game/FPSPK/Pickups/BP_Projectile.BP_Projectile_C" (Math|Transform|MakeTransform (Transformation|GetSocketLocation (Variables|Character|GetMesh) "GunSocket") (Pawn|GetControlRotation :!class /Script/Engine.Pawn) "1.000000,1.000000,1.000000") "AdjustIfPossibleButDontSpawnIfColliding" "MultiplyWithRoot" 0 self))))

(fn ConstructionScript)

(fn UpdateWalkSpeed
  (params (NewWalkSpeed :type Float%20%28double-precision%29))
  (Variables|/Script/Engine.CharacterMovementComponent|SetMaxWalkSpeed (Variables|Character|GetCharacterMovement) NewWalkSpeed))

(fn ShootPlayer
  (Animation|PlayAnimMontage "/Game/FPSPK/Enemies/MonsterBear/Animations/AM_EnemyCharacter_Gunplay_Montage.AM_EnemyCharacter_Gunplay_Montage" 1.0 "None"))